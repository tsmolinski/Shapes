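; BP_ShapesSpawner is an actor Blueprint that provides a function for spawning randomized primitive shapes inside a box volume.
; SpawnShapeRandomLocSizeColor_2 picks a class from the passed array, wrapping the index by modulo, and returns the spawned actor.
; Location is random within BoxComponent's bounds, and scale is random but uniform across axes.
; Despite the name, it sets no color, and BeginPlay and the construction script are empty.
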(event `self.ReceiveBeginPlay`)

(fn `SpawnShapeRandomLocSizeColor_2`
  (params (PrimitivesArray :type "Array of ShpsBaseShape Class Reference") (PrmitveIndex :type Integer))
  (returns (Shape :type "ShpsBaseShape Object Reference"))
  (bind _boxcomponent (`self.BoxComponent`))
  (bind _returnvalue (`|SpawnActorFromClass` (`|GetArrayItem` PrimitivesArray (mod PrmitveIndex (`KismetArrayLibrary.Array_Length` PrimitivesArray))) (`KismetMathLibrary.MakeTransform` (`KismetMathLibrary.RandomPointInBoundingBox` (`SceneComponent.K2_GetComponentLocation` _boxcomponent) (`BoxComponent.BoxExtent` _boxcomponent)) (struct) (`KismetMathLibrary.Conv_DoubleToVector` (`KismetMathLibrary.RandomFloatInRange` 0.5 2.5))) "Undefined" "MultiplyWithRoot" null null))
  (return _returnvalue))

(fn `UserConstructionScript`)